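; BP_Enemy is an enemy actor that damages the player on contact and awards score when shot.
; All logic runs from the Hit event: contact with BP_Player lowers its health, updates its health bar, then destroys the enemy, or shows the restart screen if health reaches zero.
; A BP_Projectile hit adds score to the first BP_Player found via GetAllActorsOfClass and destroys the enemy.
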(event EventBeginPlay)

(event Collision|EventActorBeginOverlap
  (params (OtherActor :type Actor%20Object%20Reference)))

(event EventTick
  (params (DeltaSeconds :type Float%20%28single-precision%29)))

(event Collision|EventHit
  (params (MyComp :type Primitive%20Component%20Object%20Reference) (Other :type Actor%20Object%20Reference) (OtherComp :type Primitive%20Component%20Object%20Reference) (bSelfMoved :type Boolean) (HitLocation :type Vector :default "0, 0, 0") (HitNormal :type Vector :default "0, 0, 0") (NormalImpulse :type Vector :default "0, 0, 0") (Hit :type Hit%20Result%20Structure%20%28by%20ref%29))
  (Utilities|FlowControl|Sequence
    (:then_0
      (bind _asbp_player (Utilities|Casting|CastToBP_Player Other))
      (bind _output_get (Variables|/Game/InfiniteMatrix/Blueprints/BP_Player.BP_Player_C|SetHealth _asbp_player (Math|Integer|Max(Integer) (- (Variables|/Game/InfiniteMatrix/Blueprints/BP_Player.BP_Player_C|GetHealth _asbp_player) 20))))
      (Default|UpdateHealthBar (Variables|/Game/InfiniteMatrix/Blueprints/BP_Player.BP_Player_C|GetHealthWidget _asbp_player) _output_get)
      (Math|Integer|CompareInt _output_get
        (:>
          (Actor|DestroyActor))
        (:==
          (Default|DisplayRestart _asbp_player))))
    (:then_1
      (Utilities|Casting|CastToBP_Projectile Other)
      (bind _outactors (Actor|GetAllActorsOfClass "/Game/InfiniteMatrix/Blueprints/BP_Player.BP_Player_C"))
      (Variables|/Game/InfiniteMatrix/Blueprints/BP_Player.BP_Player_C|SetScore (Utilities|Array|Get(acopy) _outactors) (+ (Variables|/Game/InfiniteMatrix/Blueprints/BP_Player.BP_Player_C|GetScore (Utilities|Array|Get(acopy) _outactors)) 10))
      (Actor|DestroyActor))))

(fn ConstructionScript)
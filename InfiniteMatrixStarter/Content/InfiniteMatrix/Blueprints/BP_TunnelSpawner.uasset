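; BP_TunnelSpawner builds a chain of BP_Tunnel segments, with occasional enemies and health packs.
; On BeginPlay it clears existing projectiles, enemies, pickups and tunnels, then lays initial segments starting at the player pawn.
; Each new segment attaches at the newest one's SpawnPoint, receives a spawner reference and randomizes its wall.
; A one-in-three roll adds both a short-lived enemy and health pack at random points ahead.
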(event EventBeginPlay
  (CallFunction|SpawnInitialTunnels))

(event EventTick
  (params (DeltaSeconds :type Float%20%28single-precision%29)))

(fn ConstructionScript)

(fn SpawnTunnel
  (params (SpawnLocation :type Vector))
  (bind _returnvalue (+ SpawnLocation "1250.000000,0.000000,0.000000"))
  (bind _returnvalue_2 (Game|SpawnActorfromClass "/Game/InfiniteMatrix/Blueprints/BP_Tunnel.BP_Tunnel_C" (Math|Transform|MakeTransform SpawnLocation "0, 0, 0" "1,1,1") "Undefined" 0 0))
  (bind _output_get (Variables|Default|SetNewestTunnel _returnvalue_2))
  (Variables|/Game/InfiniteMatrix/Blueprints/BP_Tunnel.BP_Tunnel_C|SetTunnelSpawner _output_get self)
  (Default|RandomizeWall _output_get)
  (if (not (Math|Conversions|ToBoolean(Integer) (Math|Random|RandomInteger 3)))
    (bind _returnvalue_3 (Game|SpawnActorfromClass "/Game/InfiniteMatrix/Blueprints/BP_HealthPack.BP_HealthPack_C" (Math|Transform|MakeTransform (Math|Random|RandomPointinBoundingBox _returnvalue "200.000000,350.000000,350.000000") "0, 0, 0" "1,1,1") "Undefined" 0 0))
    (Actor|SetLifeSpan _returnvalue_3 8.0)
    (bind _returnvalue_4 (Game|SpawnActorfromClass "/Game/InfiniteMatrix/Blueprints/BP_Enemy.BP_Enemy_C" (Math|Transform|MakeTransform (Math|Random|RandomPointinBoundingBox _returnvalue "200.000000,300.000000,300.000000") "0, 0, 0" "1.500000,1.500000,1.500000") "Undefined" 0 0))
    (Actor|SetLifeSpan _returnvalue_4 8.0)))

(fn SpawnTunnelatSpawnPoint
  (CallFunction|SpawnTunnel (Transformation|GetWorldLocation (Variables|/Game/InfiniteMatrix/Blueprints/BP_Tunnel.BP_Tunnel_C|GetSpawnPoint (Variables|Default|GetNewestTunnel)))))

(fn SpawnInitialTunnels
  (Utilities|FlowControl|Sequence
    (:then_0
      (bind _outactors (Actor|GetAllActorsOfClass "/Game/InfiniteMatrix/Blueprints/BP_Projectile.BP_Projectile_C"))
      (for _array_element _outactors
        (Actor|DestroyActor _array_element)))
    (:then_1
      (bind _outactors_2 (Actor|GetAllActorsOfClass "/Game/InfiniteMatrix/Blueprints/BP_Enemy.BP_Enemy_C"))
      (for _array_element_2 _outactors_2
        (Actor|DestroyActor _array_element_2)))
    (:then_2
      (bind _outactors_3 (Actor|GetAllActorsOfClass "/Game/InfiniteMatrix/Blueprints/BP_HealthPack.BP_HealthPack_C"))
      (for _array_element_3 _outactors_3
        (Actor|DestroyActor _array_element_3)))
    (:then_3
      (bind _outactors_4 (Actor|GetAllActorsOfClass "/Game/InfiniteMatrix/Blueprints/BP_Tunnel.BP_Tunnel_C"))
      (for _array_element_4 _outactors_4
        (Actor|DestroyActor _array_element_4)))
    (:then_4
      (for _index (range 0 2)
        (Utilities|IsValid (Variables|Default|GetNewestTunnel)
          (:Is%20Valid
            (CallFunction|SpawnTunnelatSpawnPoint))
          (:Is%20Not%20Valid
            (CallFunction|SpawnTunnel (Transformation|GetActorLocation (Game|Player|GetPlayerPawn 0)))))))))